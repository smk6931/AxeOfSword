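; BP_Boss is a boss character that carries a sword and plays an attack montage.
; On BeginPlay it spawns Bp_Sword, attaches it to the right-hand socket and caches a reference to BP_Player.
; The BoxTrace event starts a timeline that box-traces ahead with debug drawing each update and stores the hit.
; The following branch is hard-wired true, so the delayed attack montage plays regardless of the trace result.
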(event Custom|BoxTrace
  (bind _returnvalue (Transformation|GetActorLocation))
  (Timeline|Timeline PlayFromStart
    (:Update
      (bind (_outhit _returnvalue_2) (Collision|BoxTraceByChannel _returnvalue (+ _returnvalue (* (Transformation|GetActorForwardVector) 1e+02)) "40.000000,40.000000,40.000000" "0, 0, 0" "TraceTypeQuery1" false 0 "ForOneFrame"))
      (Variables|Default|SetBlocking%20Hit _returnvalue_2)
      (if true
        (Utilities|FlowControl|Delay 1.2)
        (Animation|Montage|PlayMontage (Variables|Character|GetMesh) "/Game/Boss_MK/Animation/AM_BS_Attack.AM_BS_Attack")))))

(event EventBeginPlay
  (bind _returnvalue (Game|SpawnActorfromClass "/Game/Boss_MK/Bp_Sword.Bp_Sword_C" (Transformation|GetSocketTransform (Variables|Character|GetMesh) "hand_rSocket" "RTS_World") "Undefined" "MultiplyWithRoot" 0 0))
  (Transformation|AttachComponentToComponent _returnvalue (Variables|Character|GetMesh) "hand_rSocket" "SnapToTarget" "SnapToTarget" "SnapToTarget" true)
  (bind _returnvalue_2 (Actor|GetActorOfClass "/Game/Boss_MK/BP_Player.BP_Player_C"))
  (Variables|Default|SetBp_Player _returnvalue_2))

(fn ConstructionScript)