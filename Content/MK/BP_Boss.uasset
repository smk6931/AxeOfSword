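; BP_Boss is a boss enemy that chases the player with a sword.
; BeginPlay spawns Bp_Sword and attaches it to the mesh's Grib socket.
; Every Tick issues AI MoveTo, then immediately draws a debug forward box trace without waiting for arrival.
; A branch fixed to true ignores the trace result and leads through a delay to a Play Montage call with no montage set.
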(event EventTick
  (params (DeltaSeconds :type Float%20%28single-precision%29))
  (bind _returnvalue (Transformation|GetActorLocation))
  (AI|AIMoveTo self "0, 0, 0" (Game|GetPlayerCharacter 0) 1e+02 false
    (:then
      (bind (_outhit _returnvalue_2) (Collision|BoxTraceByChannel _returnvalue (+ _returnvalue (* (Transformation|GetActorForwardVector) 1e+02)) "40.000000,40.000000,40.000000" "0, 0, 0" "TraceTypeQuery1" false 0 "ForOneFrame"))
      (Variables|Default|SetBlocking%20Hit _returnvalue_2)
      (if true
        (Utilities|FlowControl|Delay 1.2)
        (Animation|Montage|PlayMontage (Variables|Character|GetMesh) 0)))))

(event EventBeginPlay
  (bind _returnvalue (Game|SpawnActorfromClass "/Game/MK/Bp_Sword.Bp_Sword_C" (Transformation|GetSocketTransform (Variables|Character|GetMesh) "Grib" "RTS_World") "Undefined" "MultiplyWithRoot" 0 0))
  (Transformation|AttachComponentToComponent _returnvalue (Variables|Character|GetMesh) "Grib" "SnapToTarget" "SnapToTarget" "SnapToTarget" true))

(fn ConstructionScript)